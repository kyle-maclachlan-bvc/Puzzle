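; BP_Door1 is a hinged door that swings open or closed on interaction unless it is locked.
; Interaction calls OpenDoor, which prints the lock state, plays a locked-handle or creak sound, and, when unlocked, toggles DoorOpen.
; A Timeline plays or reverses to lerp the actor's rotation between the Door component's starting rotation and a 90-degree yaw offset cached at BeginPlay.
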(event `self.ReceiveBeginPlay`
  (bind (_originlocation_roll _originlocation_pitch _originlocation_yaw) (`KismetMathLibrary.BreakRotator` (`self.OriginLocation`)))
  (set `self.OriginLocation` (`SceneComponent.K2_GetComponentRotation` (`self.Door`)))
  (set `self.OpenedLocation` (`KismetMathLibrary.MakeRotator` 0.0 0.0 (+ _originlocation_yaw 90.0))))

(event `OpeningDoor`
  (bind (_direction _rotationtrack) (`Timeline|Timeline` :!label _label)
    (:`Update`
      (`self.K2_SetActorRotation` (`KismetMathLibrary.RLerp` (`self.OriginLocation`) (`self.OpenedLocation`) _rotationtrack)))))

(event `ClosingDoor`
  (goto _label :!via `Reverse`))

(event `/Game/Blueprint/BPI_Interact.Interaction`
  (`self.OpenDoor`))

(fn `OpenDoor`
  (bind _sfx (`self.SFX`))
  (bind _sfx_2 (`self.SFX`))
  (if (`self.Is Door Locked`)
    (`KismetSystemLibrary.PrintString` "Door is Locked" true true (struct :`R` 0.686686 :`G` 0.090842 :`B` 0.467784 :`A` 1.0) 2.0 "Locked")
    (`AudioComponent.SetSound` _sfx_2 "/Game/Audio/SFX/SFX_InspectorJ_-_Household_-_Locked_Door_Trying_to_Enter_Handle.SFX_InspectorJ_-_Household_-_Locked_Door_Trying_to_Enter_Handle")
    (`AudioComponent.Play` _sfx_2 0.0)
    (else
      (`KismetSystemLibrary.PrintString` "Door is Unlocked" true true (struct :`R` 0.686686 :`G` 0.090842 :`B` 0.467784 :`A` 1.0) 2.0 "Locked")
      (`AudioComponent.SetSound` _sfx "/Game/Audio/SFX/SFX_John_Silke_-_Haunted_House_-_Wooden_Door_Creaks_.SFX_John_Silke_-_Haunted_House_-_Wooden_Door_Creaks_")
      (`AudioComponent.Play` _sfx 0.0)
      (if (`self.Door Open`)
        (`KismetSystemLibrary.PrintString` "Door Open")
        (`self.OpeningDoor`)
        (else
          (`KismetSystemLibrary.PrintString` "Door Closed")
          (`self.ClosingDoor`)))
      (set `self.Door Open` (not (`self.Door Open`))))))

(fn `UserConstructionScript`)