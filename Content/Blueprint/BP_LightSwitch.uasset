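; BP_LightSwitch is an interactable switch that toggles the point lights of its linked LightSource actors.
; Trigger overlaps notify the actor's BPC_InteractionWidget component and track that actor.
; A Delay-throttled Tick shows the prompt widget only while that actor faces the switch, using a dot-product test.
; Interaction calls ToggleLight, which plays a sound, swaps the switch material and sets light visibility.
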(event `self.ReceiveTick`
  (params (DeltaSeconds :type "Float (single-precision)"))
  (bind _interactionactor (`self.InteractionActor`))
  (`KismetSystemLibrary.Delay` 0.2)
  (`/Engine/EditorBlueprintResources/StandardMacros.IsValid` (`self.InteractionActor`)
    (:`Is Valid`
      (`SceneComponent.SetVisibility` (`self.Widget`) (select `bool` (>= (`KismetMathLibrary.Dot_VectorVector` (`self.GetActorForwardVector` _interactionactor) (`KismetMathLibrary.Normal` (- (`SceneComponent.K2_GetComponentLocation` (`self.SwitchMesh`)) (`self.K2_GetActorLocation` _interactionactor)))) 0.6) :`true` true) false))
    (:`Is Not Valid`
      (`SceneComponent.SetVisibility` (`self.Widget`) false false))))

(event `self.Light_Trigger.OnComponentBeginOverlap`
  (params (OverlappedComponent :type "PrimitiveComponent Object Reference") (OtherActor :type "Actor Object Reference") (OtherComp :type "PrimitiveComponent Object Reference") (OtherBodyIndex :type Integer) (bFromSweep :type Boolean) (SweepResult :type "HitResult Structure (by ref)"))
  (bind _returnvalue (`self.GetComponentByClass` OtherActor "/Game/BPC_InteractionWidget.BPC_InteractionWidget_C"))
  (`/Engine/EditorBlueprintResources/StandardMacros.IsValid` _returnvalue
    (:`Is Valid`
      (`/Game/BPC_InteractionWidget.FN_CanInteract` _returnvalue)
      (set `self.InteractionActor` OtherActor)
      (`self.SetActorTickEnabled` true))))

(event `self.Light_Trigger.OnComponentEndOverlap`
  (params (OverlappedComponent :type "PrimitiveComponent Object Reference") (OtherActor :type "Actor Object Reference") (OtherComp :type "PrimitiveComponent Object Reference") (OtherBodyIndex :type Integer))
  (bind _returnvalue (`self.GetComponentByClass` OtherActor "/Game/BPC_InteractionWidget.BPC_InteractionWidget_C"))
  (`/Engine/EditorBlueprintResources/StandardMacros.IsValid` _returnvalue
    (:`Is Valid`
      (`/Game/BPC_InteractionWidget.FN_CanInteract` _returnvalue)
      (`self.SetActorTickEnabled` true)
      (set `self.InteractionActor` null))))

(event `/Game/Blueprint/BPI_Interact.Interaction`
  (params (Interactor :type "Actor Object Reference"))
  (`self.ToggleLight`))

(fn `GetInteractionPrompt`
  (returns (PromptText :type Text))
  (return ""))

(fn `ToggleLight`
  (bind _switchmesh (`self.SwitchMesh`))
  (bind _sfx (`self.SFX`))
  (`AudioComponent.SetSound` _sfx "/Engine/VREditor/Sounds/VR_open.VR_open")
  (`AudioComponent.Play` _sfx 0.0)
  (if (`self.SwitchOn`)
    (`PrimitiveComponent.SetMaterial` _switchmesh 0 "/Game/Materials/MI_White.MI_White")
    (else
      (`PrimitiveComponent.SetMaterial` _switchmesh 0 "/Game/Materials/MI_Red.MI_Red")))
  (set `self.SwitchOn` (not (`self.SwitchOn`)))
  (for _array_element (`self.LightSource`)
    (`SceneComponent.SetVisibility` (`/Game/Blueprint/BP_LightSource.PointLight` _array_element) (`self.SwitchOn`) false)))

(fn `UserConstructionScript`)