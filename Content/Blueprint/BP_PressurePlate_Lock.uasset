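; BP_PressurePlate_Lock is a puzzle pressure plate that tracks its state as Empty, Red, Blue or Player.
; SetNewState stores the state and shows the bad indicator material for Empty, the good one otherwise.
; When the last overlapping actor leaves, the plate resets to Empty; a following BP_PuzzleKey cast leads nowhere.
; GetCurrentState exposes the state, but nothing in this graph sets an occupied state.
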(event `self.Plate.OnComponentEndOverlap`
  (params (OverlappedComponent :type "PrimitiveComponent Object Reference") (OtherActor :type "Actor Object Reference") (OtherComp :type "PrimitiveComponent Object Reference") (OtherBodyIndex :type Integer))
  (if (`KismetArrayLibrary.Array_IsEmpty` (`PrimitiveComponent.GetOverlappingActors` (`self.Plate`) null))
    (`self.SetNewState` "NewEnumerator1")
    (cast `/Game/InteractionSystem/BP_PuzzleKey` OtherActor)))

(fn `GetCurrentState`
  (returns (`Current State` :type Byte))
  (return (`self.CurrentState`)))

(fn `SetNewState`
  (params (CurrentState :type "/Game/Blueprint/E_PressurePlateStates Enum" :default "NewEnumerator0"))
  (bind _output_get (set `self.CurrentState` CurrentState))
  (switch `/Game/Blueprint/E_PressurePlateStates` _output_get
    (:`NewEnumerator1`
      (`PrimitiveComponent.SetMaterial` (`self.Plate`) 0 "/Game/Materials/MI_Indicator_Bad.MI_Indicator_Bad"))
    (:`NewEnumerator2`
      (`PrimitiveComponent.SetMaterial` (`self.Plate`) 0 "/Game/Materials/MI_Indicator_Good.MI_Indicator_Good" :!label _label))
    (:`NewEnumerator3`
      (goto _label))
    (:`NewEnumerator4`
      (goto _label))))

(fn `UserConstructionScript`)