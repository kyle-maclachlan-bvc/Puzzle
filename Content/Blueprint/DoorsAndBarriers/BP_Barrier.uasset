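; BP_Barrier is a barrier that opens while enough pressure switches are active.
; SwitchActivated and SwitchDeactivated events raise or lower an active-switch count and compare it to the number needed.
; The OpenBarrier timeline plays when the threshold is met and reverses otherwise, driving the Cube's relative Z position.
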(event `SwitchActivated`
  (bind _result (`/Engine/EditorBlueprintResources/StandardMacros.IncrementInt` (`self.PressureSwitchesActive`))
    (:`  `
      (if (>= _result (`self.PressureSwitchesNeeded`))
        (bind (_direction _barrierposition) (`Timeline|OpenBarrier` :!label _label)
          (:`Update`
            (`SceneComponent.K2_SetRelativeLocation` (`self.Cube`) (`KismetMathLibrary.MakeVector` 0.0 0.0 _barrierposition) false false)))
        (else
          (goto _label :!via `Reverse`))))))

(event `SwitchDeactivated`
  (bind _result (`/Engine/EditorBlueprintResources/StandardMacros.DecrementInt` (`self.PressureSwitchesActive`))
    (:`  `
      (if (>= _result (`self.PressureSwitchesNeeded`))
        (goto _label)
        (else
          (goto _label :!via `Reverse`))))))

(fn `UserConstructionScript`)