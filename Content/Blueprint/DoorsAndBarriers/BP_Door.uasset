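; Interactive swinging door that the player opens and closes, spending a collected key when it is locked.
; OpenDoor checks the lock, plays the matching sound and runs a Timeline forward or in reverse to lerp the actor's yaw.
; An overlap on the icon widget records the interacting actor, and Tick shows the prompt only while that actor faces the door.
; Open state persists by DoorID in the game instance's save and is restored on BeginPlay.
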(event `self.ReceiveTick`
  (params (DeltaSeconds :type "Float (single-precision)"))
  (bind _interactionactor (`self.InteractionActor`))
  ; Widget Position for Interactivity
  (`KismetSystemLibrary.Delay` 0.2)
  (`/Engine/EditorBlueprintResources/StandardMacros.IsValid` (`self.InteractionActor`)
    (:`Is Valid`
      (`SceneComponent.SetVisibility` (`self.Widget`) (select `bool` (>= (`KismetMathLibrary.Dot_VectorVector` (`self.GetActorForwardVector` _interactionactor) (`KismetMathLibrary.Normal` (- (`SceneComponent.K2_GetComponentLocation` (`self.Door`)) (`self.K2_GetActorLocation` _interactionactor)))) 0.6) :`true` true) false))
    (:`Is Not Valid`
      (`SceneComponent.SetVisibility` (`self.Widget`) false false))))

(event `self.Icon_Widget.OnComponentBeginOverlap`
  (params (OverlappedComponent :type "PrimitiveComponent Object Reference") (OtherActor :type "Actor Object Reference") (OtherComp :type "PrimitiveComponent Object Reference") (OtherBodyIndex :type Integer) (bFromSweep :type Boolean) (SweepResult :type "HitResult Structure (by ref)"))
  (bind _returnvalue (`self.GetComponentByClass` OtherActor "/Game/BPC_InteractionWidget.BPC_InteractionWidget_C"))
  ; Display Widget on Door for Ineractivity
  (`/Engine/EditorBlueprintResources/StandardMacros.IsValid` _returnvalue
    (:`Is Valid`
      (`/Game/BPC_InteractionWidget.FN_CanInteract` _returnvalue)
      (set `self.InteractionActor` OtherActor)
      (`self.SetActorTickEnabled` true))))

(event `self.Icon_Widget.OnComponentEndOverlap`
  (params (OverlappedComponent :type "PrimitiveComponent Object Reference") (OtherActor :type "Actor Object Reference") (OtherComp :type "PrimitiveComponent Object Reference") (OtherBodyIndex :type Integer))
  (bind _returnvalue (`self.GetComponentByClass` OtherActor "/Game/BPC_InteractionWidget.BPC_InteractionWidget_C"))
  ; Hide Widget on Door for Interactvity
  (`/Engine/EditorBlueprintResources/StandardMacros.IsValid` _returnvalue
    (:`Is Valid`
      (`/Game/BPC_InteractionWidget.FN_CanInteract` _returnvalue)
      (`self.SetActorTickEnabled` true)
      (set `self.InteractionActor` null))))

(event `self.ReceiveBeginPlay`
  (bind (_originlocation_roll _originlocation_pitch _originlocation_yaw) (`KismetMathLibrary.BreakRotator` (`self.OriginLocation`)))
  (`|ExecutionSequence`
    (:`then_0`
      ; Saves the state of the Door Open or Closed
      (bind _aswb_my_game_instance (cast `/Game/Saving/WB_MyGameInstance` (`GameplayStatics.GetGameInstance`)))
      (add `/Game/Saving/WB_MyGameInstance.OnGameSaved` _aswb_my_game_instance (`|CreateDelegate` :!event `SaveDoorOpen`))
      (if (`KismetArrayLibrary.Array_Contains` (`/Game/Saving/WB_SaveGame.DoorUnlocked` (`/Game/Saving/WB_MyGameInstance.SaveRef` _aswb_my_game_instance)) (`self.DoorID`))
        (set `self.Is Door Locked` false)
        (`self.OpenDoor`)))
    (:`then_1`
      ; Sets Door to Closed Position for Animation
      (set `self.OriginLocation` (`SceneComponent.K2_GetComponentRotation` (`self.Door`)))
      (set `self.OpenedLocation` (`KismetMathLibrary.MakeRotator` 0.0 0.0 (- _originlocation_yaw 90.0))))))

(event `OpeningDoor`
  ; Animation for the Door Opening and Closing
  (bind (_direction _rotationtrack) (`Timeline|Timeline` :!label _label)
    (:`Update`
      (`self.K2_SetActorRotation` (`KismetMathLibrary.RLerp` (`self.OriginLocation`) (`self.OpenedLocation`) _rotationtrack)))))

(event `ClosingDoor`
  ; Animation for the Door Opening and Closing
  (goto _label :!via `Reverse`))

(event `/Game/Blueprint/BPI_Interact.Interaction`
  (params (Interactor :type "Actor Object Reference"))
  ; Animation for the Door Opening and Closing
  (`self.OpenDoor`))

(event `SaveDoorOpen`
  (bind _doorid (`self.DoorID`))
  ; Steps to Saving the Door State
  (bind _aswb_my_game_instance (cast `/Game/Saving/WB_MyGameInstance` (`GameplayStatics.GetGameInstance`)))
  (if (`self.Door Open`)
    (if (`self.Is Door Locked`)
      (set `self.Is Door Locked` false))
    (bind _doorunlocked (`/Game/Saving/WB_SaveGame.DoorUnlocked` (`/Game/Saving/WB_MyGameInstance.SaveRef` _aswb_my_game_instance)))
    (`KismetArrayLibrary.Array_AddUnique` _doorunlocked _doorid)
    (else
      (`KismetArrayLibrary.Array_RemoveItem` _doorunlocked _doorid))))

(fn `GetInteractionPrompt`
  (returns (PromptText :type Text))
  (return ""))

(fn `OpenDoor`
  (bind _sfx (`self.SFX`))
  (bind _sfx_2 (`self.SFX`))
  (bind _sfx_3 (`self.SFX`))
  (if (`self.Is Door Locked`)
    (if (> (`/Game/ThirdPerson/Blueprints/BP_ThirdPersonCharacter.KeyCollected` (cast `/Game/ThirdPerson/Blueprints/BP_ThirdPersonCharacter` (`GameplayStatics.GetPlayerPawn` 0) :!pure true)) 0)
      ; Door is Closed and Locked, BUT Player has a Key
      (bind _asbp_third_person_character (cast `/Game/ThirdPerson/Blueprints/BP_ThirdPersonCharacter` (`GameplayStatics.GetPlayerPawn` 0)))
      (`/Engine/EditorBlueprintResources/StandardMacros.DecrementInt` (`/Game/ThirdPerson/Blueprints/BP_ThirdPersonCharacter.KeyCollected` _asbp_third_person_character)
        (:`  `
          (set `self.Is Door Locked` (not (`self.Is Door Locked`)))
          (`AudioComponent.SetSound` _sfx_3 "/Game/Audio/SFX/SC_UnlockDoor.SC_UnlockDoor")
          (`AudioComponent.Play` _sfx_3 0.0)
          ; Runs Opening Door Animation or Closing Door Animation
          (if (`self.Door Open`) :!label _label
            (`self.ClosingDoor`)
            (else
              (`self.OpeningDoor`)))
          (set `self.Door Open` (not (`self.Door Open`)))))
      (else
        ; Door is Closed and Locked
        (`AudioComponent.SetSound` _sfx_2 "/Game/Audio/SFX/SFX_LockedDoor.SFX_LockedDoor")
        (`AudioComponent.Play` _sfx_2 0.0)))
    (else
      ; Door is closed and unlocked
      (`AudioComponent.SetSound` _sfx "/Game/Audio/SFX/SC_DoorSound.SC_DoorSound")
      (`AudioComponent.Play` _sfx 0.0)
      (goto _label))))

(fn `UserConstructionScript`)