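; Interactable hinged door that swings 90 degrees in yaw and can be locked.
; Interaction calls OpenDoor, which plays a locked sound if locked, otherwise plays the door sound and alternates between opening and closing events.
; A timeline plays forward or in reverse to lerp the whole actor's rotation between the Door's rotation at BeginPlay and the offset rotation.
; The interaction prompt is empty.
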(event `self.ReceiveBeginPlay`
  (bind (_originlocation_roll _originlocation_pitch _originlocation_yaw) (`KismetMathLibrary.BreakRotator` (`self.OriginLocation`)))
  (set `self.OriginLocation` (`SceneComponent.K2_GetComponentRotation` (`self.Door`)))
  (set `self.OpenedLocation` (`KismetMathLibrary.MakeRotator` 0.0 0.0 (+ _originlocation_yaw 90.0))))

(event `OpeningDoor`
  (bind (_direction _rotationtrack) (`Timeline|Timeline` :!label _label)
    (:`Update`
      (`self.K2_SetActorRotation` (`KismetMathLibrary.RLerp` (`self.OriginLocation`) (`self.OpenedLocation`) _rotationtrack)))))

(event `ClosingDoor`
  (goto _label :!via `Reverse`))

(event `/Game/Blueprint/BPI_Interact.Interaction`
  (params (Interactor :type "Actor Object Reference"))
  (`self.OpenDoor`))

(fn `GetInteractionPrompt`
  (returns (PromptText :type Text))
  (return ""))

(fn `OpenDoor`
  (bind _sfx (`self.SFX`))
  (bind _sfx_2 (`self.SFX`))
  (if (`self.Is Door Locked`)
    (`AudioComponent.SetSound` _sfx_2 "/Game/Audio/SFX/SFX_LockedDoor.SFX_LockedDoor")
    (`AudioComponent.Play` _sfx_2 0.0)
    (else
      (`AudioComponent.SetSound` _sfx "/Game/Audio/SFX/SC_DoorSound.SC_DoorSound")
      (`AudioComponent.Play` _sfx 0.0)
      (if (`self.Door Open`)
        (`self.OpeningDoor`)
        (else
          (`self.ClosingDoor`)))
      (set `self.Door Open` (not (`self.Door Open`))))))

(fn `UserConstructionScript`)