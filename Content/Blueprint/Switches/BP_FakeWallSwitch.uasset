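; BP_FakeWallSwitch is an interactable switch that toggles a linked fake wall, with an empty interaction prompt.
; Each interaction plays a sound, swaps the switch mesh between white and red materials, and notifies FakeWallToOpen of activation or deactivation based on SwitchOn.
; It then flips SwitchOn and applies the new value to the point light visibility of every element in an array.
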(event `self.Interaction`
  (params (Interactor :type "Actor Object Reference"))
  (`self.ToggleFakeWall`))

(fn `GetInteractionPrompt`
  (returns (PromptText :type Text))
  (return ""))

(fn `ToggleFakeWall`
  (bind _fakewalltoopen (`self.FakeWallToOpen`))
  (bind _sfx (`self.SFX`))
  (bind _switchmesh (`self.SwitchMesh`))
  (`AudioComponent.SetSound` _sfx "/Engine/VREditor/Sounds/VR_open.VR_open")
  (`AudioComponent.Play` _sfx 0.0)
  (if (`self.SwitchOn`)
    (`PrimitiveComponent.SetMaterial` _switchmesh 0 "/Game/Materials/MI_White.MI_White")
    (`/Game/Blueprint/DoorsAndBarriers/BP_FakeWall.SwitchActivated` _fakewalltoopen)
    (else
      (`PrimitiveComponent.SetMaterial` _switchmesh 0 "/Game/Materials/MI_Red.MI_Red")
      (`/Game/Blueprint/DoorsAndBarriers/BP_FakeWall.SwitchDeactivated` _fakewalltoopen)))
  (set `self.SwitchOn` (not (`self.SwitchOn`)))
  ; Opens Fake Wall and Provides access to set up multiple fake walls on one switch
  (for _array_element _
    (`SceneComponent.SetVisibility` (`/Game/Blueprint/BP_LightSource.PointLight` _array_element) (`self.SwitchOn`) false)))

(fn `UserConstructionScript`)