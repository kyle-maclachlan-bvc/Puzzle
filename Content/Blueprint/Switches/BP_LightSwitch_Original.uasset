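; BP_LightSwitch_Original is an interactable wall or prop switch that turns a set of linked lights on and off.
; The Interaction event calls ToggleLight, which plays a sound, swaps the switch mesh material (red when on, white when off) and flips SwitchOn.
; It then applies that state to the PointLight visibility of every entry in the LightSource array.
; Its interaction prompt is an empty string.
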(event `self.Interaction`
  (params (Interactor :type "Actor Object Reference"))
  (`self.ToggleLight`))

(fn `GetInteractionPrompt`
  (returns (PromptText :type Text))
  (return ""))

(fn `ToggleLight`
  (bind _switchmesh (`self.SwitchMesh`))
  (bind _sfx (`self.SFX`))
  (`AudioComponent.SetSound` _sfx "/Engine/VREditor/Sounds/VR_open.VR_open")
  (`AudioComponent.Play` _sfx 0.0)
  (if (`self.SwitchOn`)
    (`PrimitiveComponent.SetMaterial` _switchmesh 0 "/Game/Materials/MI_White.MI_White")
    (else
      (`PrimitiveComponent.SetMaterial` _switchmesh 0 "/Game/Materials/MI_Red.MI_Red")))
  (set `self.SwitchOn` (not (`self.SwitchOn`)))
  (for _array_element (`self.LightSource`)
    (`SceneComponent.SetVisibility` (`/Game/Blueprint/BP_LightSource.PointLight` _array_element) (`self.SwitchOn`) false)))

(fn `UserConstructionScript`)