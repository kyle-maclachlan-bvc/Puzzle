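; BP_PressurePlate_Keys is a weighted pressure plate that reveals a puzzle key while a BP_CubeWeight overlaps it.
; On BeginPlay it spawns the key at Spawnpoint, hidden and without collision.
; Overlap begin and end toggle the key's visibility and hitbox through KeyVisibility.
; With a valid linked indicator light, they also switch it green or red, swap the switch material and play or reverse the switch movement timeline.
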(event `self.ReceiveBeginPlay`
  (bind _returnvalue (`|SpawnActorFromClass` "/Game/InteractionSystem/BP_PuzzleKey.BP_PuzzleKey_C" (`SceneComponent.K2_GetComponentToWorld` (`self.spawnpoint`)) "AdjustIfPossibleButAlwaysSpawn" "MultiplyWithRoot" null null))
  (set `self.SpawnedKey` _returnvalue)
  (`self.KeyVisibility` false))

(event `self.ReceiveActorBeginOverlap`
  (params (OtherActor :type "Actor Object Reference"))
  (bind _indicatorlighttochange (`self.IndicatorLightToChange`))
  (cast `/Game/InteractionSystem/BP_CubeWeight` OtherActor)
  (`self.KeyVisibility` true)
  (`/Engine/EditorBlueprintResources/StandardMacros.IsValid` _indicatorlighttochange
    (:`Is Valid`
      (`/Game/Blueprint/BP_SwitchIndicator.GreenIndicator` _indicatorlighttochange)
      (`PrimitiveComponent.SetMaterial` (`self.Switch`) 0 "/Game/Materials/MI_Indicator_Good.MI_Indicator_Good")
      (bind (_direction _switchposition) (`Timeline|SwitchActivate` :!label _label)
        (:`Update`
          (`SceneComponent.K2_SetRelativeLocation` (`self.Switch`) (`KismetMathLibrary.MakeVector` 0.0 0.0 _switchposition) false false))))))

(event `self.ReceiveActorEndOverlap`
  (params (OtherActor :type "Actor Object Reference"))
  (bind _indicatorlighttochange (`self.IndicatorLightToChange`))
  (cast `/Game/InteractionSystem/BP_CubeWeight` OtherActor)
  (`/Engine/EditorBlueprintResources/StandardMacros.IsValid` (`self.SpawnedKey`)
    (:`Is Valid`
      (`self.KeyVisibility` false)
      (`/Engine/EditorBlueprintResources/StandardMacros.IsValid` _indicatorlighttochange
        (:`Is Valid`
          (`/Game/Blueprint/BP_SwitchIndicator.RedIndicator` _indicatorlighttochange)
          (`PrimitiveComponent.SetMaterial` (`self.Switch`) 0 "/Game/Materials/MI_Indicator_Bad.MI_Indicator_Bad")
          (goto _label :!via `Reverse`))))))

(fn `KeyVisibility`
  (params (Visible :type Boolean))
  (bind _spawnedkey (`self.SpawnedKey`))
  (bind _hitbox (`/Game/InteractionSystem/BP_PuzzleKey.HitBox` _spawnedkey))
  (`SceneComponent.SetVisibility` (`/Game/InteractionSystem/BP_PuzzleKey.DefaultSceneRoot` _spawnedkey) Visible true)
  (if Visible
    (`PrimitiveComponent.SetCollisionEnabled` _hitbox "QueryAndPhysics")
    (else
      (`PrimitiveComponent.SetCollisionEnabled` _hitbox "NoCollision"))))

(fn `UserConstructionScript`)