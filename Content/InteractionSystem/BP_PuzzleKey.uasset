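; BP_PuzzleKey is a collectible key pickup that adds to the player's key count.
; When an actor overlaps its HitBox and the BP_Key reference is valid, it casts that actor to BP_ThirdPersonCharacter and increments KeyCollected directly on the character.
; It then spawns the NS_Burst effect at the key base, plays a 2D collection sound and destroys itself.
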(event `self.HitBox.OnComponentBeginOverlap`
  (params (OverlappedComponent :type "PrimitiveComponent Object Reference") (OtherActor :type "Actor Object Reference") (OtherComp :type "PrimitiveComponent Object Reference") (OtherBodyIndex :type Integer) (bFromSweep :type Boolean) (SweepResult :type "HitResult Structure (by ref)"))
  (`/Engine/EditorBlueprintResources/StandardMacros.IsValid` "/Game/Blueprint/BP_Key.BP_Key"
    (:`Is Valid`
      (bind _asbp_third_person_character (cast `/Game/ThirdPerson/Blueprints/BP_ThirdPersonCharacter` OtherActor))
      (bind _result (`/Engine/EditorBlueprintResources/StandardMacros.IncrementInt` (`/Game/ThirdPerson/Blueprints/BP_ThirdPersonCharacter.KeyCollected` _asbp_third_person_character))
        (:`  `
          (set `/Game/ThirdPerson/Blueprints/BP_ThirdPersonCharacter.KeyCollected` _result _asbp_third_person_character)
          (`NiagaraFunctionLibrary.SpawnSystemAtLocation` "/Game/VFX/NS_Burst.NS_Burst" (`SceneComponent.K2_GetComponentLocation` (`self.KeyBase`)))
          (`GameplayStatics.PlaySound2D` (`self.SFX to Collect`) 1.0 1.0 0.0 null null)
          (`self.K2_DestroyActor`))))))

(fn `NewFunction`)

(fn `UserConstructionScript`)